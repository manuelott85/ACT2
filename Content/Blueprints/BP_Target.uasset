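; BP_Target is a target that falls over when it takes any damage, then stands back up after a reset delay.
; A hit plays audio and sets a target rotation offset 90 degrees in roll from the saved initial one, while a gate blocks further hits until reset.
; Tick interpolates the rotation root with RInterpTo at separate falling and rising speeds, updating only until the target rotation is reached.
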(event `self.ReceiveBeginPlay`
  ;[1 1 1] BeginPlay
  ;[1 1 1] Save initial rotation
  (set `self.InitialRotation` (`SceneComponent.RelativeRotation` (`self.RotationRoot`))))

(event `self.ReceiveAnyDamage`
  (params (Damage :type "Float (single-precision)") (DamageType :type "DamageType Object Reference") (InstigatedBy :type "Controller Object Reference") (DamageCauser :type "Actor Object Reference"))
  (bind (_initialrotation_roll _initialrotation_pitch _initialrotation_yaw) (`KismetMathLibrary.BreakRotator` (`self.InitialRotation`)))
  ;[1 1 1] EventAnyDmg
  (`/Engine/EditorBlueprintResources/StandardMacros.Gate` false :!label _label
    (:`Exit`
      (set `self.TargetRotation` (`KismetMathLibrary.MakeRotator` (+ _initialrotation_roll -90.0) _initialrotation_pitch _initialrotation_yaw))
      (set `self.TargetSpeed` (`self.SpeedFalling`))
      (set `self.bShouldUpdate` true)
      (`|ExecutionSequence`
        (:`then_0`
          ;[1 1 1] Play Audio
          (`AudioComponent.Play` (`self.Audio`) 0.0)
          (goto _label :!via `Close`))
        (:`then_1`
          (`KismetSystemLibrary.Delay` (`self.ResetTime`))
          (set `self.TargetRotation` (`self.InitialRotation`))
          (set `self.TargetSpeed` (`self.SpeedStandingUp`))
          (set `self.bShouldUpdate` true)
          (goto _label :!via `Open`))))))

(event `self.ReceiveTick`
  (params (DeltaSeconds :type "Float (single-precision)"))
  ;[1 1 1] EventTick
  ;[1 1 1] Only update if needed
  (if (`self.bShouldUpdate`)
    ;[1 1 1] Animate
    (`SceneComponent.K2_SetRelativeRotation` (`self.RotationRoot`) (`KismetMathLibrary.RInterpTo` (`SceneComponent.RelativeRotation` (`self.RotationRoot`)) (`self.TargetRotation`) (`GameplayStatics.GetWorldDeltaSeconds`) (`self.TargetSpeed`)) false false)
    ;[1 1 1] Stop animating if in final position
    (if (== (`SceneComponent.RelativeRotation` (`self.RotationRoot`)) (`self.TargetRotation`) :`ErrorTolerance` 0.01)
      (set `self.bShouldUpdate` false))))

(fn `UserConstructionScript`)