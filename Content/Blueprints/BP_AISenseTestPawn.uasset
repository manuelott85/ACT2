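; Test pawn for an AI vision sense that turns to face the player's pawn every tick and views it through a scene capture.
; On BeginPlay it creates its own small render target for the capture and shows it on its plane through a dynamic material.
; CalculatePixels averages the target's red channel as a white-pixel measure and prints it, but its visible call is disconnected.
; AlterFoV only prints a distance-based interpolation.
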(event `CreateIndividualRenderTargetAndMaterialInstance`
  (bind _plane (`self.Plane`))
  ;[1 1 1] Create a new render target & assign it to the SceneCapture2D; create a new material instance and set the render target as source texture
  (bind _returnvalue (`KismetRenderingLibrary.CreateRenderTarget2D` 128 128 "RTF_RGBA8"))
  (set `SceneCaptureComponent2D.TextureTarget` _returnvalue (`self.SceneCaptureComponent2D`))
  (bind _returnvalue_2 (`PrimitiveComponent.CreateDynamicMaterialInstance` _plane 0 (`PrimitiveComponent.GetMaterial` _plane 0) "None"))
  (`MaterialInstanceDynamic.SetTextureParameterValue` _returnvalue_2 "RenderTarget" _returnvalue)
  (`PrimitiveComponent.SetMaterial` _plane 0 _returnvalue_2))

(event `AlterFoV`
  (params (Target :type "Actor Object Reference"))
  (`KismetSystemLibrary.PrintString` (`KismetStringLibrary.Conv_VectorToString` (`KismetMathLibrary.VLerp` (170.0 1000.0 0.0) (20.0 67000.0 0.0) (/ (`KismetMathLibrary.VSize` (- (`self.K2_GetActorLocation`) (`self.K2_GetActorLocation` Target))) 67000.0)))))

(event `self.ReceiveBeginPlay`
  (set `SceneCaptureComponent2D.FOVAngle` 60.0 (`self.SceneCaptureComponent2D`))
  (`self.CreateIndividualRenderTargetAndMaterialInstance`))

(event `self.ReceiveTick`
  (params (DeltaSeconds :type "Float (single-precision)"))
  (`self.K2_SetActorRotation` (`KismetMathLibrary.FindLookAtRotation` (`self.K2_GetActorLocation`) (`self.K2_GetActorLocation` (`Controller.K2_GetPawn` (`GameplayStatics.GetPlayerController` 0))))))

(event `CalculatePixels`
  (bind _texturetarget (`SceneCaptureComponent2D.TextureTarget` (`self.SceneCaptureComponent2D`)))
  (set `self.numberWhitePixel` 0.0)
  (`/Engine/EditorBlueprintResources/StandardMacros.IsValid` _texturetarget
    (:`Is Valid`
      ;[1 1 1] Read out every pixel
      (bind _returnvalue (`FunctionLibrary.getAverageValueFromAllColors` _texturetarget))
      ;[1 1 1] Count each NOT black pixel
      (for _array_element _returnvalue
        (set `self.numberWhitePixel` (+ (`self.numberWhitePixel`) (`KismetMathLibrary.Conv_ByteToDouble` (`.R` (break `Color` _array_element))))))
      (set `self.numberWhitePixel` (/ (`self.numberWhitePixel`) (`KismetMathLibrary.Conv_IntToDouble` (* (`TextureRenderTarget2D.SizeX` _texturetarget) (`TextureRenderTarget2D.SizeY` _texturetarget)))))
      (`KismetSystemLibrary.PrintString` (`KismetStringLibrary.Conv_DoubleToString` (`self.numberWhitePixel`)) true false (struct :`G` 0.66 :`B` 1.0 :`A` 1.0) (* (`GameplayStatics.GetWorldDeltaSeconds`) 2.0)))))

(fn `UserConstructionScript`)