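; Custom player camera manager that moves an ACTCharacter's view onto the primary weapon's sight when aiming down sights.
; BlueprintUpdateCamera projects the first-person camera position onto the SightSocket's forward axis with a dot product, keeping its depth along that axis.
; It lerps toward that point by AimAlpha, using control rotation and a fixed FOV.
; The non-aiming branch computes a negated-alpha location but returns no override.
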(fn `BlueprintUpdateCamera`
  (params (CameraTarget :type "Actor Object Reference"))
  (returns (NewCameraLocation :type "Vector Structure") (NewCameraRotation :type "Rotator Structure") (NewCameraFOV :type "Float (double-precision)") (ReturnValue :type Boolean))
  (bind _asactcharacter (cast `ACTCharacter` CameraTarget))
  (`/Engine/EditorBlueprintResources/StandardMacros.IsValid` _asactcharacter
    (:`Is Valid`
      (bind _primaryweapon (`ACTCharacter.PrimaryWeapon` _asactcharacter))
      (`/Engine/EditorBlueprintResources/StandardMacros.IsValid` _primaryweapon
        (:`Is Valid`
          (set `self.FinalCameraRotation` (`Pawn.GetControlRotation` _asactcharacter))
          (if (`ACTCharacter.bAimsDownSights` _asactcharacter)
            (bind _returnvalue (`SceneComponent.K2_GetComponentLocation` (`ACTCharacter.FirstPersonCamera` _asactcharacter)))
            (bind (_returnvalue_location _returnvalue_rotation) (`KismetMathLibrary.BreakTransform` (`SceneComponent.GetSocketTransform` (`Weapon_Base.weaponAsset` _primaryweapon) "SightSocket" "RTS_World")))
            (bind _returnvalue_2 (`KismetMathLibrary.GetForwardVector` _returnvalue_rotation))
            (bind _returnvalue_3 (- _returnvalue_location _returnvalue))
            (bind _returnvalue_4 (- _returnvalue_location (* _returnvalue_2 (* (`KismetMathLibrary.Dot_VectorVector` (`KismetMathLibrary.Normal` _returnvalue_3) _returnvalue_2) (`KismetMathLibrary.VSize` _returnvalue_3)))))
            (bind _aimalpha (`ACTCharacter.aimAlpha` _asactcharacter))
            (set `self.FinalCameraLocation` (`KismetMathLibrary.VLerp` _returnvalue _returnvalue_4 _aimalpha))
            (return (`self.FinalCameraLocation`) (`self.FinalCameraRotation`) 90.0 true)
            (else
              (set `self.FinalCameraLocation` (`KismetMathLibrary.VLerp` _returnvalue _returnvalue_4 (* _aimalpha -1.0))))))))))

(fn `UserConstructionScript`)